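; Lighting and environment rig that pairs an HDRI sky dome with four rect lights (one key, three fill) and can shuffle to a random HDRI.
; Construction and BeginPlay rebuild lights, capture FOVs, post process and dome, centering the light pivot on an optional focus actor.
; A dynamic material receives the HDRI, image adjustments and yaw-driven rotation.
; A self-resetting Shuffle bool triggers randomization, drawing from a fallback array when the main one is empty.
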(event `self.ReceiveBeginPlay`
  (`self.Construct_Shuffler`))

(fn `Construct_Shuffler`
  (bind (_location _rotation) (`self.Get_Lights_Loc_Rot`))
  (bind _rectlightc (`self.RectLightC`))
  (bind _skydome_mat (`self.SkyDome_mat`))
  (bind _skydome (`self.SkyDome`))
  (bind _capture_fov (`self.Capture_FOV`))
  (bind _rectlightc_2 (`self.RectLightC`))
  (bind _rectlighta (`self.RectLightA`))
  (bind _light_pivot (`self.light_pivot`))
  (bind (_returnvalue_roll _returnvalue_pitch _returnvalue_yaw) (`KismetMathLibrary.BreakRotator` (`SceneComponent.K2_GetComponentRotation` (`self.DefaultSceneRoot`))))
  (set `SceneCaptureComponent2D.FOVAngle` _capture_fov (`self.Capture_A_2D`))
  (set `SceneCaptureComponent2D.FOVAngle` _capture_fov (`self.Capture_D_2D`))
  (set `SceneCaptureComponent2D.FOVAngle` _capture_fov (`self.Capture_C_2D`))
  (set `SceneCaptureComponent2D.FOVAngle` _capture_fov (`self.Capture_B_2D`))
  (`SceneComponent.K2_SetWorldLocation` (`self.Offset_D`) (+ (`SceneComponent.K2_GetComponentLocation` (`self.light_pivot`)) (`KismetMathLibrary.MakeVector` 0.0 0.0 (`self.Light_Height_Offset`))) false false)
  (`SceneComponent.K2_SetWorldLocation` (`self.Offset_C`) (+ (`SceneComponent.K2_GetComponentLocation` (`self.light_pivot`)) (`KismetMathLibrary.MakeVector` 0.0 0.0 (`self.Light_Height_Offset`))) false false)
  (`SceneComponent.K2_SetWorldLocation` (`self.Offset_A`) (+ (`SceneComponent.K2_GetComponentLocation` (`self.light_pivot`)) (`KismetMathLibrary.MakeVector` 0.0 0.0 (`self.Light_Height_Offset`))) false false)
  (`SceneComponent.K2_SetWorldLocation` (`self.Offset_B`) (+ (`SceneComponent.K2_GetComponentLocation` (`self.light_pivot`)) (`KismetMathLibrary.MakeVector` 0.0 0.0 (`self.Light_Height_Offset`))) false false)
  (`SceneComponent.K2_SetRelativeLocationAndRotation` (`self.RectLightA`) _location _rotation false false)
  (`SceneComponent.K2_SetRelativeLocationAndRotation` (`self.RectLightB`) _location _rotation false false)
  (`SceneComponent.K2_SetRelativeLocationAndRotation` (`self.RectLightC`) _location _rotation false false)
  (`RectLightComponent.SetBarnDoorLength` _rectlightc (`self.Barn_Door_Length`))
  (`RectLightComponent.SetBarnDoorLength` (`self.RectLightB`) (`self.Barn_Door_Length`))
  (`RectLightComponent.SetBarnDoorLength` (`self.RectLightA`) (`self.Barn_Door_Length`))
  (`RectLightComponent.SetBarnDoorLength` (`self.RectLightD`) (`self.Barn_Door_Length`))
  (`RectLightComponent.SetBarnDoorAngle` _rectlightc (`self.Barn_Door_Angle`))
  (`RectLightComponent.SetBarnDoorAngle` (`self.RectLightD`) (`self.Barn_Door_Angle`))
  (`RectLightComponent.SetBarnDoorAngle` (`self.RectLightB`) (`self.Barn_Door_Angle`))
  (`RectLightComponent.SetBarnDoorAngle` (`self.RectLightA`) (`self.Barn_Door_Angle`))
  (`RectLightComponent.SetSourceHeight` _rectlightc (`self.Barn_Door_Height`))
  (`RectLightComponent.SetSourceHeight` (`self.RectLightB`) (`self.Barn_Door_Height`))
  (`RectLightComponent.SetSourceHeight` (`self.RectLightA`) (`self.Barn_Door_Height`))
  (`SceneComponent.K2_SetRelativeLocation` (`self.RectLightD`) (`self.Get_Lights_Loc_Rot`) false false)
  (`LightComponent.SetIntensity` _rectlighta (`self.Key_Intensity`))
  (`LocalLightComponent.SetAttenuationRadius` _rectlighta (`self.KeyAttenuation`))
  (`LightComponent.SetIntensity` _rectlightc_2 (`self.Fill_Intensity`))
  (`LightComponent.SetIntensity` (`self.RectLightB`) (`self.Fill_Intensity`))
  (`LightComponent.SetIntensity` (`self.RectLightD`) (`self.Fill_Intensity`))
  (`LocalLightComponent.SetAttenuationRadius` _rectlightc_2 (`self.FillAttenuation`))
  (`LocalLightComponent.SetAttenuationRadius` (`self.RectLightB`) (`self.FillAttenuation`))
  (`LocalLightComponent.SetAttenuationRadius` (`self.RectLightD`) (`self.FillAttenuation`))
  (if (`KismetSystemLibrary.IsValid` (`self.Light_Focus_Actor`))
    (`SceneComponent.K2_SetRelativeRotation` _light_pivot (`KismetMathLibrary.MakeRotator` (.roll (`SceneComponent.RelativeRotation` _light_pivot)) (.pitch (`SceneComponent.RelativeRotation` _light_pivot)) (+ (.yaw (`SceneComponent.RelativeRotation` _light_pivot)) (`self.Light_Turn_Offset`))) false false)
    (`SceneComponent.K2_SetWorldLocation` (`self.light_pivot`) (`self.Character_Shuffler_Bounds`) false false))
  (set `PostProcessComponent.Settings` (`self.Post Process Settings`) (`self.PostProcess`))
  ;[1 1 1] skydome sm size
  (`SceneComponent.SetWorldScale3D` (`self.SkyDome`) (`KismetMathLibrary.Conv_DoubleToVector` (`self.Sky_Size`)))
  ;[1 1 1] init rotation start
  (if (`KismetSystemLibrary.IsValid` _skydome_mat)
    (`|ExecutionSequence`
      (:`then_0`
        (for _array_element (`MaterialInstance.ScalarParameterValues` _skydome_mat)
          (if (== (break `MaterialParameterInfo` (break `ScalarParameterValue` _array_element)) "Rotation")
            (set `self.HDRIStartRotation` (`.ParameterValue` (break `ScalarParameterValue` _array_element))))))
      (:`then_1`
        ;[1 1 1] mat creation
        (`PrimitiveComponent.SetMaterial` _skydome 0 _skydome_mat)
        ;[1 1 1] mat dynamic instance & apply to static mesh
        (bind _returnvalue (`PrimitiveComponent.CreateDynamicMaterialInstance` _skydome 0 _skydome_mat "None"))
        (set `self.SkyDome_mat_dyn` _returnvalue)
        ;[1 1 1] set up the hdri and set the tex cube in the material
        (`self.Get_Set_HDRI_Safe`)
        (`self.Set_HDRI_Mat_Param_Efficient`)
        (for (_array_element_2 _array_index) (`|MakeArray` (`self.Exposure`) (`self.Power`) (`self.Saturation`))
          (`MaterialInstanceDynamic.SetScalarParameterValue` (`self.SkyDome_mat_dyn`) (`|GetArrayItem` (`|MakeArray` "Exposure" "Power" "Saturation") _array_index) _array_element_2))
        ;[1 1 1] update rotation based on bp rot z
        (`MaterialInstanceDynamic.SetScalarParameterValue` (`self.SkyDome_mat_dyn`) "Rotation" (+ (`self.HDRIStartRotation`) (/ _returnvalue_yaw -360.0)))))))

(fn `Set_HDRI_Mat_Param`
  (set `self.HDRI` (`|GetArrayItem` (`self.HDRI_Safe_Array`) (`KismetMathLibrary.Clamp` (`self.HDRI_Idx`) 0 (`self.idx_max`))))
  (`MaterialInstanceDynamic.SetTextureParameterValue` (`self.SkyDome_mat_dyn`) "HDRI" (`self.HDRI`)))

(fn `Set_HDRI_Mat_Param_Efficient`
  (set `self.HDRI` (`|GetArrayItem` (`self.HDRI_Safe_Array`) (`KismetMathLibrary.Clamp` (`self.HDRI_Idx`) 0 (`self.idx_max`))))
  (`MaterialInstanceDynamic.SetTextureParameterValue` (`self.SkyDome_mat_dyn`) "HDRI" (`self.HDRI`)))

(fn `Shuffle!`
  ;[1 1 1] Make sure tex arrays are legit
  (`self.Get_Set_HDRI_Safe`)
  ;[1 1 1] Choose rand tex from legit arrays
  (set `self.HDRI_Idx` (`KismetMathLibrary.RandomIntegerInRange` 0 (`self.idx_max`)))
  ;[1 1 1] get the hdri at the index, set it safely in mat param
  (`self.Set_HDRI_Mat_Param_Efficient`)
  (`self.Construct_Shuffler`))

(fn `UserConstructionScript`
  (`self.Construct_Shuffler`)
  (if (`self.Shuffle`)
    (set `self.Shuffle` false)
    (`self.Shuffle!`)))